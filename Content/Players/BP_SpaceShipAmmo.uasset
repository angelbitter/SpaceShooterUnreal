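; BP_SpaceShipAmmo is a laser projectile, evidently fired by the player's spaceship, that plays a firing sound when it spawns.
; It moves itself forward every tick at Speed using unswept location updates.
; Overlapping an actor tagged Enemy triggers a one-time explosion effect and sound, then destroys the projectile after a short delay.
; Overlapping a "Muro" (wall) actor destroys it immediately, and no damage is applied here.
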(event `self.ReceiveActorBeginOverlap`
  (params (OtherActor :type "Actor Object Reference"))
  (bind _tags (`Actor.Tags` OtherActor))
  (if (and (not (`self.HasCollided`)) (`KismetArrayLibrary.Array_Contains` _tags "Enemy"))
    (set `self.HasCollided` true)
    (`GameplayStatics.SpawnEmitterAtLocation` "/Game/StarterContent/Particles/P_Explosion.P_Explosion" (`self.K2_GetActorLocation`))
    (`GameplayStatics.PlaySound2D` "/Game/StarterContent/Audio/Explosion02.Explosion02" 0.2 2.0 0.0 null null)
    (`KismetSystemLibrary.Delay` 0.2)
    (`self.K2_DestroyActor`)
    (elif (`KismetArrayLibrary.Array_Contains` _tags "Muro")
      (`self.K2_DestroyActor`))))

(event `self.ReceiveBeginPlay`
  (`GameplayStatics.PlaySound2D` "/Engine/VREditor/Sounds/UI/Laser_Pull.Laser_Pull" 1.0 1.0 0.0 null null))

(event `self.ReceiveTick`
  (params (DeltaSeconds :type "Float (single-precision)"))
  (`self.K2_SetActorLocation` (+ (`self.K2_GetActorLocation`) (* (`self.GetActorForwardVector`) (* (`self.Speed`) DeltaSeconds)))))

(fn `UserConstructionScript`)