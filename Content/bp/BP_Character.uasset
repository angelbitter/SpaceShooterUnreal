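; Player character that rotates, moves along its forward axis and spawns Ammo at FirePoint, with a timer limiting fire rate.
; Overlapping a "Muro" actor wraps it across the arena by negating out-of-bounds X or Y.
; "Enemy" overlaps restart timer-driven mesh blinking and, if vulnerable, remove a life and grant brief invulnerability.
; At zero lives it notifies BP_GameMode and destroys itself.
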(event `self.ReceiveActorBeginOverlap`
  (params (OtherActor :type "Actor Object Reference"))
  (bind _tags (`Actor.Tags` OtherActor))
  (if (`KismetArrayLibrary.Array_Contains` _tags "Muro")
    (`self.ChangeLocation`)
    (set `self.Changing` false)
    (elif (`KismetArrayLibrary.Array_Contains` _tags "Enemy")
      (`self.DamageActor`))))

(event `DamageActor`
  (`self.TimerVisibilityOn`)
  (if (`self.IsVulnerable`)
    (set `self.IsVulnerable` false)
    (`GameplayStatics.PlaySound2D` "/Engine/VREditor/Sounds/UI/Leave_Simulate.Leave_Simulate" 1.0 1.0 0.0 null null)
    (bind _output_get (set `self.Lifes` (- (`self.Lifes`) 1)))
    (if (== _output_get 0)
      (bind _asbp_game_mode (cast `/Game/bp/BP_GameMode` (`GameplayStatics.GetGameMode`)))
      (`/Game/bp/BP_GameMode.PlayerDead` _asbp_game_mode)
      (`self.K2_DestroyActor`)
      (else
        (`KismetSystemLibrary.Delay` (`self.VulnerabilityTime`))
        (set `self.IsVulnerable` true)))))

(event `EnhancedInput|/Game/input/BP_InputFire`
  (params (ActionValue :type Boolean) (ElapsedSeconds :type "Float (double-precision)") (TriggeredSeconds :type "Float (double-precision)") (InputAction :type "InputAction Object Reference" :default "/Game/input/BP_InputFire.BP_InputFire"))
  (:`Triggered`
    (if (`self.CanFire`)
      (`self.Do FIre`)
      (set `self.CanFire` false)
      (`KismetSystemLibrary.K2_SetTimerDelegate` (delegate `UpdateFire`) (`self.FireDelay`)))))

(event `UpdateFire`
  (set `self.CanFire` true))

(event `EnhancedInput|/Game/input/BP_InputMove`
  (params (ActionValue :type "Vector2D Structure") (ElapsedSeconds :type "Float (double-precision)") (TriggeredSeconds :type "Float (double-precision)") (InputAction :type "InputAction Object Reference" :default "/Game/input/BP_InputMove.BP_InputMove"))
  (:`Triggered`
    (`self.AddMovementInput` (`self.GetActorForwardVector`) ActionValue_Y)))

(event `EnhancedInput|/Game/input/BP_InputRotateLeft`
  (params (ActionValue :type Boolean) (ElapsedSeconds :type "Float (double-precision)") (TriggeredSeconds :type "Float (double-precision)") (InputAction :type "InputAction Object Reference" :default "/Game/input/BP_InputRotateLeft.BP_InputRotateLeft"))
  (:`Triggered`
    (`self.K2_AddActorLocalRotation` (`KismetMathLibrary.MakeRotator` 0.0 0.0 (* (`GameplayStatics.GetWorldDeltaSeconds`) (* (`self.rotation speed`) -1.0))))))

(event `self.ReceiveBeginPlay`
  (bind _asplayer_controller (cast `PlayerController` (`self.GetController`)))
  (bind _returnvalue (pcsubsystem `EnhancedInputLocalPlayerSubsystem` _asplayer_controller))
  (`/Engine/EditorBlueprintResources/StandardMacros.IsValid` _returnvalue
    (:`Is Valid`
      (`EnhancedInputSubsystemInterface.AddMappingContext` _returnvalue "/Game/input/BP_InputMapping.BP_InputMapping" 0 (struct)))))

(event `EnhancedInput|/Game/input/BP_InputRotateRight`
  (params (ActionValue :type Boolean) (ElapsedSeconds :type "Float (double-precision)") (TriggeredSeconds :type "Float (double-precision)") (InputAction :type "InputAction Object Reference" :default "/Game/input/BP_InputRotateRight.BP_InputRotateRight"))
  (:`Triggered`
    (`self.K2_AddActorLocalRotation` (`KismetMathLibrary.MakeRotator` 0.0 0.0 (* (`GameplayStatics.GetWorldDeltaSeconds`) (`self.rotation speed`))))))

(fn `ChangeLocation`
  (bind _x (.x (`self.K2_GetActorLocation`)))
  (bind _y (.y (`self.K2_GetActorLocation`)))
  (bind _z (.z (`self.K2_GetActorLocation`)))
  (bind _returnvalue (* _y -1.0))
  (bind _returnvalue_2 (* _x -1.0))
  (bind _returnvalue_3 (and (> _y -1000.0) (< _y 1000.0)))
  (if (not (`self.Changing`))
    (set `self.Changing` true)
    (if (and (> _x -500.0) (< _x 500.0))
      (if _returnvalue_3
        (`self.K2_SetActorLocation` (`KismetMathLibrary.MakeVector` _x _y _z) false true)
        (else
          (`self.K2_SetActorLocation` (`KismetMathLibrary.MakeVector` _x _returnvalue _z) false true)))
      (elif _returnvalue_3
        (`self.K2_SetActorLocation` (`KismetMathLibrary.MakeVector` _returnvalue_2 _y _z) false true)
        (else
          (`self.K2_SetActorLocation` (`KismetMathLibrary.MakeVector` _returnvalue_2 _returnvalue _z) false true))))))

(fn `Do FIre`
  (`|SpawnActorFromClass` (`self.Ammo`) (`SceneComponent.K2_GetComponentToWorld` (`self.FirePoint`)) "Undefined" "MultiplyWithRoot" null null))

(fn `TimerVisibilityOff`
  (`KismetSystemLibrary.K2_ClearTimer` null "ToggleVisibility")
  (`SceneComponent.SetVisibility` (`self.Mesh`) true false))

(fn `TimerVisibilityOn`
  (`KismetSystemLibrary.K2_SetTimer` null "ToggleVisibility" 0.2 true)
  (`KismetSystemLibrary.K2_SetTimer` null "TimerVisibilityOff" (`self.VulnerabilityTime`)))

(fn `ToggleVisibility`
  (if (`SceneComponent.IsVisible` (`self.Mesh`))
    (`SceneComponent.SetVisibility` (`self.Mesh`) false false)
    (else
      (`SceneComponent.SetVisibility` (`self.Mesh`) true false))))

(fn `UserConstructionScript`)