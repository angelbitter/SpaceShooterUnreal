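; Tougher basic enemy in a spaceship shooter that loses one HP per player shot.
; Overlaps with PlayerShot-tagged ammo decrement HP; at zero it hides its mesh, passes 1000 to the game mode's EnemyDestroyed, then fires OnEnemyDestroy after a short delay.
; Overlaps with "Muro" (wall) actors call ChangeLocation, then clear the Changing flag after a brief delay.
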(event `self.ReceiveActorBeginOverlap`
  (params (OtherActor :type "Actor Object Reference"))
  (bind _tags (`Actor.Tags` OtherActor))
  (if (`KismetArrayLibrary.Array_Contains` _tags "PlayerShot")
    (cast `/Game/Players/BP_SpaceShipAmmo` OtherActor)
    (bind _output_get (set `self.HP` (- (`self.HP`) 1)))
    (if (<= _output_get 0)
      (`SceneComponent.SetVisibility` (`self.Mesh`) false false)
      (bind _asbp_game_mode (cast `/Game/bp/BP_GameMode` (`GameplayStatics.GetGameMode`)))
      (`/Game/bp/BP_GameMode.EnemyDestroyed` _asbp_game_mode 1000)
      (`KismetSystemLibrary.Delay` 0.2)
      (`self.OnEnemyDestroy`))
    (elif (`KismetArrayLibrary.Array_Contains` _tags "Muro")
      (`self.ChangeLocation`)
      (`KismetSystemLibrary.Delay` 0.1)
      (set `self.Changing` false))))

(fn `UserConstructionScript`
  (`parent.UserConstructionScript`))