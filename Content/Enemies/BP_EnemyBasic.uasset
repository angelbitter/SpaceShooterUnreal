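; Basic enemy actor that flies straight along its initial forward vector and dies when overlapped by a PlayerShot.
; A hit passes a point value to BP_GameMode, hides the mesh and, after brief delays, destroys the actor through its OnEnemyDestroy event.
; Overlapping a "Muro" actor wraps it across the arena by negating out-of-bounds X/Y, with a Changing flag as debounce.
; Tick resets a shot timer, but Fire, which spawns Ammo at FirePoint, is disconnected.
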(event `self.ReceiveBeginPlay`
  (set `self.MovementVector` (`self.GetActorForwardVector`))
  (add `self.OnEnemyDestroy` (delegate `Destroyed_Event`)))

(event `Destroyed_Event`
  (`KismetSystemLibrary.Delay` 0.2)
  (`self.K2_DestroyActor`))

(event `self.ReceiveActorBeginOverlap`
  (params (OtherActor :type "Actor Object Reference"))
  (bind _tags (`Actor.Tags` OtherActor))
  (if (`KismetArrayLibrary.Array_Contains` _tags "PlayerShot")
    (bind _asbp_game_mode (cast `/Game/bp/BP_GameMode` (`GameplayStatics.GetGameMode`)))
    (`/Game/bp/BP_GameMode.EnemyDestroyed` _asbp_game_mode 250)
    (`SceneComponent.SetVisibility` (`self.Mesh`) false false)
    (`KismetSystemLibrary.Delay` 0.2)
    (`self.OnEnemyDestroy`)
    (elif (`KismetArrayLibrary.Array_Contains` _tags "Muro")
      (`self.ChangeLocation`)
      (`KismetSystemLibrary.Delay` 0.1)
      (set `self.Changing` false))))

(event `self.ReceiveTick`
  (params (DeltaSeconds :type "Float (single-precision)"))
  (`self.Move` DeltaSeconds)
  (bind _output_get (set `self.ShootCurrentTime` (+ DeltaSeconds (`self.ShootCurrentTime`))))
  (if (> _output_get (`self.DelayShot`))
    (set `self.ShootCurrentTime` 0.0)))

(fn `ChangeLocation`
  (bind _x (.x (`self.K2_GetActorLocation`)))
  (bind _y (.y (`self.K2_GetActorLocation`)))
  (bind _z (.z (`self.K2_GetActorLocation`)))
  (bind _returnvalue (* _y -1.0))
  (bind _returnvalue_2 (* _x -1.0))
  (bind _returnvalue_3 (and (> _y -1000.0) (< _y 1000.0)))
  (if (not (`self.Changing`))
    (set `self.Changing` true)
    (if (and (> _x -500.0) (< _x 500.0))
      (if _returnvalue_3
        (`self.K2_SetActorLocation` (`KismetMathLibrary.MakeVector` _x _y _z) false true)
        (else
          (`self.K2_SetActorLocation` (`KismetMathLibrary.MakeVector` _x _returnvalue _z) false true)))
      (elif _returnvalue_3
        (`self.K2_SetActorLocation` (`KismetMathLibrary.MakeVector` _returnvalue_2 _y _z) false true)
        (else
          (`self.K2_SetActorLocation` (`KismetMathLibrary.MakeVector` _returnvalue_2 _returnvalue _z) false true))))))

(fn `Fire`
  (locals (NewLocalVar :type "Rotator Structure" :default (struct :`Yaw` 180.0)))
  (bind _returnvalue (`|SpawnActorFromClass` (`self.Ammo`) (`SceneComponent.K2_GetComponentToWorld` (`self.FirePoint`)) "Undefined" "MultiplyWithRoot" null null))
  (`self.K2_SetActorRotation` _returnvalue (`local.NewLocalVar`) false))

(fn `Move`
  (params (DeltaTime :type "Float (double-precision)"))
  (`self.K2_SetActorLocation` (+ (`self.K2_GetActorLocation`) (* (* (`self.Speed`) DeltaTime) (`self.MovementVector`)))))

(fn `UserConstructionScript`)