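; BP_EnemyAmmo is an enemy projectile that flies straight ahead and reacts to what it overlaps.
; It plays a laser sound on spawn, then Tick moves it along its forward vector by Speed without sweeping.
; Overlapping a Player-tagged actor spawns an explosion effect and sound, then destroys it after a short delay, applying no damage itself.
; Overlapping a Muro-tagged actor destroys it immediately.
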(event `self.ReceiveActorBeginOverlap`
  (params (OtherActor :type "Actor Object Reference"))
  (bind _tags (`Actor.Tags` OtherActor))
  (if (`KismetArrayLibrary.Array_Contains` _tags "Player")
    (`GameplayStatics.SpawnEmitterAtLocation` "/Game/StarterContent/Particles/P_Explosion.P_Explosion" (`self.K2_GetActorLocation`))
    (`GameplayStatics.PlaySound2D` "/Game/StarterContent/Audio/Explosion01.Explosion01" 0.4 1.0 0.0 null null)
    (`KismetSystemLibrary.Delay` 0.2)
    (`self.K2_DestroyActor`)
    (elif (`KismetArrayLibrary.Array_Contains` _tags "Muro")
      (`self.K2_DestroyActor`))))

(event `self.ReceiveBeginPlay`
  (`GameplayStatics.PlaySound2D` "/Engine/VREditor/Sounds/UI/Laser_Pull.Laser_Pull" 1.0 1.0 0.0 null null))

(event `self.ReceiveTick`
  (params (DeltaSeconds :type "Float (single-precision)"))
  (`self.K2_SetActorLocation` (+ (`self.K2_GetActorLocation`) (* (`self.GetActorForwardVector`) (* (`self.Speed`) DeltaSeconds)))))

(fn `UserConstructionScript`)