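; Enemy that chases the player in straight dashes, pausing periodically to fire a projectile at them.
; Tick moves it along a stored vector until a shot timer stops it; after a short delay FireChasing spawns aimed ammo and re-points that vector at the player, then movement resumes.
; Overlap with a PlayerShot-tagged actor awards score through BP_GameMode and triggers destruction, with a bound handler removing the actor after a brief delay.
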(event `self.ReceiveBeginPlay`
  (set `self.MovementVector_0` (`self.GetActorForwardVector`))
  (add `self.OnEnemyDestroy` (delegate `Destroyed_Event`)))

(event `Destroyed_Event`
  (`KismetSystemLibrary.Delay` 0.2)
  (`self.K2_DestroyActor`))

(event `self.ReceiveActorBeginOverlap`
  (params (OtherActor :type "Actor Object Reference"))
  (if (`KismetArrayLibrary.Array_Contains` (`Actor.Tags` OtherActor) "PlayerShot")
    (bind _asbp_game_mode (cast `/Game/bp/BP_GameMode` (`GameplayStatics.GetGameMode`)))
    (`/Game/bp/BP_GameMode.EnemyDestroyed` _asbp_game_mode 500)
    (`self.Destroyed_Event`)))

(event `self.ReceiveTick`
  (params (DeltaSeconds :type "Float (single-precision)"))
  (if (not (`self.Stopped_0`))
    (`self.MoveChasing` DeltaSeconds)
    (bind _output_get (set `self.ShootCurrentTime_0` (+ DeltaSeconds (`self.ShootCurrentTime_0`))))
    (if (> _output_get (`self.DelayShot_0`))
      (set `self.Stopped_0` true)
      (`KismetSystemLibrary.Delay` 0.5)
      (set `self.ShootCurrentTime_0` 0.0)
      (`self.FireChasing`)
      (`KismetSystemLibrary.Delay` 0.2)
      (set `self.Stopped_0` false))))

(fn `FireChasing`
  (bind _returnvalue (`KismetMathLibrary.FindLookAtRotation` (`self.K2_GetActorLocation`) (`self.K2_GetActorLocation` (`GameplayStatics.GetPlayerCharacter` 0))))
  (bind _returnvalue_2 (`|SpawnActorFromClass` (`self.Ammo_0`) (`SceneComponent.K2_GetComponentToWorld` (`self.FirePoint_0`)) "Undefined" "MultiplyWithRoot" null null))
  (`self.K2_SetActorRotation` _returnvalue_2 _returnvalue false)
  (set `self.MovementVector_0` (`KismetMathLibrary.Conv_RotatorToVector` _returnvalue)))

(fn `MoveChasing`
  (params (DeltaTime :type "Float (double-precision)"))
  (bind _output_get (set `self.MovementVector_0` (`self.MovementVector_0`)))
  (`self.K2_SetActorLocation` (+ (`self.K2_GetActorLocation`) (* (* (`self.Speed_0`) DeltaTime) _output_get))))

(fn `UserConstructionScript`)